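; Player controller for a pinball game that routes keyboard input to the flippers and plunger and manages the HUD and pause menu.
; On BeginPlay it gathers the level's flippers into left and right arrays by flip type, caches the first plunger found and adds the HUD.
; Ctrl keys flip and flop each side, Space charges and releases the plunger, and Caps Lock toggles pause with a menu widget.
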(event Custom|DetectPlunger
  (bind _outactors (Actor|GetAllActorsOfClass "/Game/BluePrints/BP_Plunger.BP_Plunger_C"))
  (Variables|Default|SetPlunger (Utilities|Array|Get(acopy) _outactors)))

(event Custom|DetectFlipper
  (bind _outactors (Actor|GetAllActorsOfClass "/Game/BluePrints/BP_Flipper.BP_Flipper_C"))
  (for _array_element _outactors
    (switch Utilities|FlowControl|Switch|SwitchonFlipType (Variables|/Game/BluePrints/BP_Flipper.BP_Flipper_C|GetFlipType _array_element)
      (:NewEnumerator0
        (Utilities|Array|Add (Variables|Default|GetLeftFlippers) _array_element))
      (:NewEnumerator1
        (Utilities|Array|Add (Variables|Default|GetRightFlippers) _array_element)))))

(event Custom|CreatePlayerHUD
  (bind _returnvalue (UserInterface|CreateWidget "/Game/BluePrints/WBP_PinballHUD.WBP_PinballHUD_C"))
  (UserInterface|Viewport|AddtoViewport _returnvalue 0))

(event EventBeginPlay
  (CallFunction|DetectFlipper)
  (CallFunction|DetectPlunger)
  (CallFunction|CreatePlayerHUD))

(event EventTick
  (params (DeltaSeconds :type Float%20%28single-precision%29)))

(event Input|KeyboardEvents|LeftCtrl
  (params (Key :type Key%20Structure :default "None"))
  (bind _leftflippers (Variables|Default|GetLeftFlippers))
  (:Pressed
    (for _array_element _leftflippers
      (Default|Flip _array_element)))
  (:Released
    (for _array_element_2 _leftflippers
      (Default|Flop _array_element_2))))

(event Input|KeyboardEvents|RightCtrl
  (params (Key :type Key%20Structure :default "None"))
  (bind _rightflippers (Variables|Default|GetRightFlippers))
  (:Pressed
    (for _array_element _rightflippers
      (Default|Flip _array_element)))
  (:Released
    (for _array_element_2 _rightflippers
      (Default|Flop _array_element_2))))

(event Input|KeyboardEvents|SpaceBar
  (params (Key :type Key%20Structure :default "None"))
  (bind _plunger (Variables|Default|GetPlunger))
  (:Pressed
    (Default|ChargePlunger _plunger))
  (:Released
    (Default|StopCharge _plunger)))

(event Input|KeyboardEvents|CapsLock
  (params (Key :type Key%20Structure :default "None"))
  (:Pressed
    (if (not (Variables|Default|GetIsPauseGame))
      (Variables|Default|SetIsPauseGame true)
      (Variables|Default|SetbShowMouseCursor true)
      (bind _returnvalue (UserInterface|CreateWidget "/Game/BluePrints/WBP_PauseGame.WBP_PauseGame_C" (Game|GetPlayerController 0)))
      (bind _output_get (Variables|Default|SetPauseMenuWidget _returnvalue))
      (UserInterface|Viewport|AddtoViewport _output_get 0)
      (Game|SetGamePaused true)
      (else
        (Variables|Default|SetIsPauseGame false)
        (Widget|RemovefromParent (Variables|Default|GetPauseMenuWidget))
        (Game|SetGamePaused false)))))

(fn ConstructionScript)