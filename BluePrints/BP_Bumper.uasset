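; BP_Bumper is a pinball bumper that kicks an overlapping BP_Ball away and awards score through BP_PinballGameMode.
; The kick is a horizontal velocity-change impulse pointing away from the bumper, scaled from the ball's speed and clamped.
; Each hit plays an attached sound and restarts the BumpLerp timeline.
; The timeline drives the mechanism's vertical offset, point light intensity and emissive boost on a dynamic material created in the construction script.
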(event Custom|Bump
  (params (Ball :type BP%20Ball%20Object%20Reference))
  (bind _returnvalue (Transformation|GetActorLocation Ball))
  (bind _returnvalue_2 (Transformation|GetActorLocation))
  (bind _returnvalue_3 (Math|Vector|GetUnitDirection(Vector) _returnvalue_2 _returnvalue))
  (bind _returnvalue_4 (Transformation|GetComponentVelocity (Variables|/Game/BluePrints/BP_Ball.BP_Ball_C|GetBall Ball)))
  (bind _returnvalue_5 (Math|Vector|VectorLength _returnvalue_4))
  (bind _returnvalue_6 (* _returnvalue_5 3.0))
  (bind _returnvalue_7 (Math|Float|Clamp(Float) _returnvalue_6 1e+02 4.5e+03))
  (bind _returnvalue_8 (* _returnvalue_3 _returnvalue_7))
  (Physics|AddImpulse (Variables|/Game/BluePrints/BP_Ball.BP_Ball_C|GetBall Ball) (Math|Vector|MakeVector (.x _returnvalue_8) (.y _returnvalue_8) 0.0) "None" true)
  (Audio|SpawnSoundAttached "/Game/Sounds/BumperHit.BumperHit" (Variables|Default|GetBumperMesh) "None" "0, 0, 0" "0, 0, 0" "KeepRelativeOffset" false 1.0 1.0 0.0 0 0)
  (bind _asbp_pinball_game_mode (Utilities|Casting|CastToBP_PinballGameMode (Game|GetGameMode))
    (:then
      (Default|AddScore _asbp_pinball_game_mode 1e+01)
      (bind _bumpalpha (Timeline|BumpLerp PlayFromStart)
        (:Update
          (Transformation|SetRelativeLocation (Variables|Default|GetBumperMechinasum) (Math|Vector|Lerp(Vector) "0, 0, 0" "0.000000,0.000000,-70.000000" _bumpalpha) false false)
          (Rendering|Components|Light|SetIntensity (Variables|Default|GetPointLight) (Math|Float|Lerp 0.0 5e+03 _bumpalpha))
          (Rendering|Material|SetScalarParameterValue (Variables|Default|GetBumperTopMid) "EmissiveBoost" (Math|Float|Lerp 0.0 2e+01 _bumpalpha) :!class /Script/Engine.MaterialInstanceDynamic))))
    (:CastFailed
      (Timeline|BumpLerp PlayFromStart))))

(event EventBeginPlay)

(event Collision|EventActorBeginOverlap
  (params (OtherActor :type Actor%20Object%20Reference))
  (bind _asbp_ball (Utilities|Casting|CastToBP_Ball OtherActor))
  (CallFunction|Bump _asbp_ball))

(event EventTick
  (params (DeltaSeconds :type Float%20%28single-precision%29)))

(fn ConstructionScript
  (bind _returnvalue (Rendering|Material|CreateDynamicMaterialInstance (Variables|Default|GetBumperMesh) 1 0 "None" :!class /Script/Engine.PrimitiveComponent))
  (Variables|Default|SetBumperTopMid _returnvalue))