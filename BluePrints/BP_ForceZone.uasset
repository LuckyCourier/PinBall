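; BP_ForceZone is a zone actor that reacts to a BP_Ball inside its Box.
; Box begin and end overlap events cast the other actor to BP_Ball and set or clear the IsBallinSide flag.
; While the flag is set, Tick applies ForceVector through AddForce on the Box component itself, not on the overlapping ball, with acceleration change off.
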(event OnComponentBeginOverlap(Box)
  (params (OverlappedComponent :type Primitive%20Component%20Object%20Reference) (OtherActor :type Actor%20Object%20Reference) (OtherComp :type Primitive%20Component%20Object%20Reference) (OtherBodyIndex :type Integer) (bFromSweep :type Boolean) (SweepResult :type Hit%20Result%20Structure%20%28by%20ref%29))
  (Utilities|Casting|CastToBP_Ball OtherActor)
  (Variables|Default|SetIsBallinSide true))

(event OnComponentEndOverlap(Box)
  (params (OverlappedComponent :type Primitive%20Component%20Object%20Reference) (OtherActor :type Actor%20Object%20Reference) (OtherComp :type Primitive%20Component%20Object%20Reference) (OtherBodyIndex :type Integer))
  (Utilities|Casting|CastToBP_Ball OtherActor)
  (Variables|Default|SetIsBallinSide false))

(event EventBeginPlay)

(event Collision|EventActorBeginOverlap
  (params (OtherActor :type Actor%20Object%20Reference)))

(event EventTick
  (params (DeltaSeconds :type Float%20%28single-precision%29))
  (if (Variables|Default|GetIsBallinSide)
    (Physics|AddForce (Variables|Default|GetBox) (Variables|Default|GetForceVector) "None" false)))

(fn ConstructionScript)