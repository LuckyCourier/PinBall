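; Pinball game mode that runs the session from main menu through ball respawns to high-score entry.
; ResetGame restores defaults, creates the HUD and spawns a ball at the plunger, and each ball's OnDestroyed event spawns the next or ends the game.
; EndGame opens high-score entry if the cached, lazily loaded save has room or the score beats its lowest.
; AddScore applies the multiplier to incoming points.
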(event Custom|SpawnBall
  (bind _outactors (Actor|GetAllActorsOfClass "/Game/BluePrints/BP_Plunger.BP_Plunger_C"))
  (bind _returnvalue (Game|SpawnActorfromClass "/Game/BluePrints/BP_Ball.BP_Ball_C" (Math|Transform|MakeTransform (Default|GetBallSpawnLocation (Utilities|Array|Get(acopy) _outactors)) "0, 0, 0" "1.000000,1.000000,1.000000") "Undefined" 0 0))
  (Game|BindEventtoOnDestroyed _returnvalue (delegate Custom|OnBallDestoryed)))

(event Custom|OnBallDestoryed
  (params (DestroyedActor :type Actor%20Object%20Reference))
  (if (> (Variables|Default|GetBallsRemaninig) 0)
    (CallFunction|SpawnBall)
    (Math|Integer|DecrementInt (Variables|Default|GetBallsRemaninig))
    (else
      (CallFunction|EndGame))))

(event Custom|EndGame
  (bind _currentsaveobject (CallFunction|GetSavedGameData))
  (if (<= (Utilities|Array|Length (Variables|/Game/BluePrints/HighScoreSave.HighScoreSave_C|GetSaveStruct _currentsaveobject)) 3)
    (CallFunction|CreateHighScoreList :!label _label)
    (else
      (bind _lowestscorestruct (Default|DeteemineLowestScoreValue _currentsaveobject))
      (if (< (.score _lowestscorestruct) (Variables|Default|GetScore))
        (goto _label)))))

(event Custom|Reset%20Game
  (bind _returnvalue (Game|GetPlayerController 0))
  (bind (_score _multiplyer _ballsremaninig) (Utilities|GetClassDefaults "BP_PinballGameMode_C"))
  (bind _asbp_pinball_player_controller (Utilities|Casting|CastToBP_PinballPlayerController _returnvalue))
  (Variables|Default|SetScore _score)
  (Variables|Default|SetMultiplyer _multiplyer)
  (Variables|Default|SetBallsRemaninig _ballsremaninig)
  (CallFunction|SpawnBall)
  (Default|CreatePlayerHUD _asbp_pinball_player_controller)
  (Variables|/Script/Engine.PlayerController|SetbShowMouseCursor _asbp_pinball_player_controller false))

(event Custom|CreateMainMenu
  (bind _returnvalue (Game|GetPlayerController 0))
  (bind _asbp_pinball_player_controller (Utilities|Casting|CastToBP_PinballPlayerController _returnvalue))
  (CallFunction|GetSavedGameData)
  (Viewport|RemoveAllWidgets)
  (bind _returnvalue_2 (UserInterface|CreateWidget "/Game/BluePrints/WBP_MainMenu.WBP_MainMenu_C" _asbp_pinball_player_controller))
  (UserInterface|Viewport|AddtoViewport _returnvalue_2 0)
  (Variables|/Script/Engine.PlayerController|SetbShowMouseCursor _asbp_pinball_player_controller true))

(event Custom|CreateHighScoreList
  (bind _returnvalue (Game|GetPlayerController 0))
  (bind _asbp_pinball_player_controller (Utilities|Casting|CastToBP_PinballPlayerController _returnvalue))
  (bind _returnvalue_2 (UserInterface|CreateWidget "/Game/BluePrints/WBP_HighScoreEntry.WBP_HighScoreEntry_C" _asbp_pinball_player_controller))
  (UserInterface|Viewport|AddtoViewport _returnvalue_2 0)
  (Variables|/Script/Engine.PlayerController|SetbShowMouseCursor _asbp_pinball_player_controller true))

(event EventBeginPlay
  (CallFunction|CreateMainMenu))

(event EventTick
  (params (DeltaSeconds :type Float%20%28single-precision%29)))

(fn ConstructionScript)

(fn AddScore
  (params (PointsToAdd :type Float%20%28double-precision%29))
  (bind _output_get (Variables|Default|SetScore (+ (* PointsToAdd (Variables|Default|GetMultiplyer)) (Variables|Default|GetScore))))
  (return _output_get))

(fn GetSavedGameData
  (bind _currentsavesobject (Variables|Default|GetCurrentSavesObject)
    (:then
      (return _currentsavesobject))
    (:else
      (bind _returnvalue (SaveGame|DoesSaveGameExist (Variables|Default|GetHighScoreSaveName)))
      (if _returnvalue
        (bind _returnvalue_2 (SaveGame|LoadGamefromSlot (Variables|Default|GetHighScoreSaveName)))
        (bind _ashigh_score_save (Utilities|Casting|CastToHighScoreSave _returnvalue_2)
          (:then
            (Default|SortSaveData _ashigh_score_save)
            (bind _output_get (Variables|Default|SetCurrentSavesObject _ashigh_score_save))
            (return _output_get))
          (:CastFailed
            _))
        (else
          (bind _returnvalue_3 (SaveGame|CreateSaveGameObject "/Game/BluePrints/HighScoreSave.HighScoreSave_C"))
          (bind _ashigh_score_save_2 (Utilities|Casting|CastToHighScoreSave _returnvalue_3)
            (:then
              (bind _output_get_2 (Variables|Default|SetCurrentSavesObject _ashigh_score_save_2))
              (return _output_get_2))
            (:CastFailed
              _))))
      (return 0))))